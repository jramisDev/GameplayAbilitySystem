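; BP_Door is a tag-gated door actor that opens by destroying itself when the player character meets its condition.
; When BP_TopDownCharacter overlaps the Box, it checks that the character's CurrentTag lacks the RoomLocked game state and contains the door's ConditionTag.
; On success it appends AdditionalGameplayEventTags to the character's tags before removal, so passing a door can grant further state.
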(event OnComponentBeginOverlap(Box)
  (params (OverlappedComponent :type Primitive%20Component%20Object%20Reference) (OtherActor :type Actor%20Object%20Reference) (OtherComp :type Primitive%20Component%20Object%20Reference) (OtherBodyIndex :type Integer) (bFromSweep :type Boolean) (SweepResult :type Hit%20Result%20Structure%20%28by%20ref%29))
  (bind _asbp_top_down_character (Utilities|Casting|CastToBP_TopDownCharacter OtherActor))
  (if (not (GameplayTags|HasTag (Variables|/Game/00_Clase/BP_TopDownCharacter.BP_TopDownCharacter_C|GetCurrentTag _asbp_top_down_character) "(TagName=\"Gameplay.GameState.RoomLocked\")"))
    (if (GameplayTags|HasTag (Variables|/Game/00_Clase/BP_TopDownCharacter.BP_TopDownCharacter_C|GetCurrentTag _asbp_top_down_character) (Variables|Default|GetConditionTag))
      (GameplayTags|AppendGameplayTagContainers (Variables|/Game/00_Clase/BP_TopDownCharacter.BP_TopDownCharacter_C|GetCurrentTag _asbp_top_down_character) (Variables|Default|GetAdditionalGameplayEventTags))
      (Actor|DestroyActor))))

(fn ConstructionScript)