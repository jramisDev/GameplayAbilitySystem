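; BP_LavaPool is a lava hazard volume that applies a configurable gameplay effect to overlapping actors.
; On box overlap, it applies EffectClass through the actor's UTHUB_ASC component and stores the returned handle per actor in the PlayerEffects map.
; On overlap end, it removes all stacks by that handle and clears the map entry, but only for BP_TopDownCharacter actors.
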(event OnComponentBeginOverlap(Box)
  (params (OverlappedComponent :type Primitive%20Component%20Object%20Reference) (OtherActor :type Actor%20Object%20Reference) (OtherComp :type Primitive%20Component%20Object%20Reference) (OtherBodyIndex :type Integer) (bFromSweep :type Boolean) (SweepResult :type Hit%20Result%20Structure%20%28by%20ref%29))
  (bind _returnvalue (Actor|GetComponentbyClass OtherActor "/Script/UTHUB_GAS_2025.UTHUB_ASC"))
  (Utilities|IsValid _returnvalue
    (:Is%20Valid
      (bind _returnvalue_2 (Class|UTHUBASC|ApplyGameplayEffect _returnvalue (Variables|Default|GetEffect%20Class)))
      (Utilities|Map|Add (Variables|Default|GetPlayerEffects) OtherActor _returnvalue_2))))

(event OnComponentEndOverlap(Box)
  (params (OverlappedComponent :type Primitive%20Component%20Object%20Reference) (OtherActor :type Actor%20Object%20Reference) (OtherComp :type Primitive%20Component%20Object%20Reference) (OtherBodyIndex :type Integer))
  (bind _returnvalue (Actor|GetComponentbyClass OtherActor "/Script/UTHUB_GAS_2025.UTHUB_ASC"))
  (bind _asbp_top_down_character (Utilities|Casting|CastToBP_TopDownCharacter OtherActor))
  (if (.ReturnValue (Utilities|Map|Find (Variables|Default|GetPlayerEffects) _asbp_top_down_character))
    (Utilities|IsValid _returnvalue
      (:Is%20Valid
        (bind _returnvalue_2 (GameplayEffects|RemoveActiveGameplayEffect _returnvalue (.Value (Utilities|Map|Find (Variables|Default|GetPlayerEffects) _asbp_top_down_character)) -1))
        (if _returnvalue_2
          (Utilities|Map|Remove (Variables|Default|GetPlayerEffects) _asbp_top_down_character))))))

(event EventBeginPlay)

(fn ConstructionScript)